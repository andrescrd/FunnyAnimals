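; Legacy player controller that switches the on-screen UI between loading, playing and complete game phases.
; Each of OnLoading, OnPlaying and OnComplete removes all widgets, creates that phase's widget and adds it to the viewport.
; Loading and complete use UI-only input, playing uses game-only input, and the mouse cursor shows only on the complete screen.
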(event EventBeginPlay)

(event EventTick
  (params (DeltaSeconds :type Float%20%28single-precision%29)))

(event EventOnComplete
  (params (InstigatorPawn :type Pawn%20Object%20Reference))
  (Viewport|RemoveAllWidgets)
  (bind _returnvalue (UserInterface|CreateWidget "/Game/UI/Gameplay/WB_Complete.WB_Complete_C"))
  (UserInterface|Viewport|AddtoViewport _returnvalue 0)
  (Input|SetInputModeUIOnly self 0 "DoNotLock")
  (Variables|Default|SetbShowMouseCursor true))

(event EventOnPlaying
  (Viewport|RemoveAllWidgets)
  (bind _returnvalue (UserInterface|CreateWidget "/Game/UI/Gameplay/WB_Player.WB_Player_C"))
  (UserInterface|Viewport|AddtoViewport _returnvalue 0)
  (Input|SetInputModeGameOnly self)
  (Variables|Default|SetbShowMouseCursor false))

(event EventOnLoading
  (Viewport|RemoveAllWidgets)
  (bind _returnvalue (UserInterface|CreateWidget "/Game/UI/AllLeves/WB_Loading.WB_Loading_C"))
  (UserInterface|Viewport|AddtoViewport _returnvalue 0)
  (Input|SetInputModeUIOnly self 0 "DoNotLock")
  (Variables|Default|SetbShowMouseCursor false))

(fn ConstructionScript)