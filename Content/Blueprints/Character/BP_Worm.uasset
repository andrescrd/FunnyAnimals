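; Worm Blueprint that colors its mesh from the bird color data table when play begins.
; GetColorFromDataTable supplies base, light and dark colors from DT_BirdColors.
; Each color feeds its own dynamic instance of M_BaseColor, which is assigned to a separate material slot on the mesh.
; Tick and the construction script are empty.
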(event EventBeginPlay
  (bind _returnvalue (Class|FBlueprintFunctionLibrary|GetColorfromDataTable "/Game/Utils/DT_BirdColors.DT_BirdColors"))
  (Utilities|FlowControl|Sequence
    (:then_0
      (bind _returnvalue_2 (Rendering|Material|CreateDynamicMaterialInstance "/Game/Assets/Materials/M_BaseColor.M_BaseColor" "None" "None" :!class /Script/Engine.KismetMaterialLibrary))
      (Rendering|Material|SetVectorParameterValue _returnvalue_2 "Color" (.colorbase _returnvalue) :!class /Script/Engine.MaterialInstanceDynamic)
      (Rendering|Material|SetMaterial (Variables|Character|GetMesh) 1 _returnvalue_2))
    (:then_1
      (bind _returnvalue_3 (Rendering|Material|CreateDynamicMaterialInstance "/Game/Assets/Materials/M_BaseColor.M_BaseColor" "None" "None" :!class /Script/Engine.KismetMaterialLibrary))
      (Rendering|Material|SetVectorParameterValue _returnvalue_3 "Color" (.colorlight _returnvalue) :!class /Script/Engine.MaterialInstanceDynamic)
      (Rendering|Material|SetMaterial (Variables|Character|GetMesh) 2 _returnvalue_3))
    (:then_2
      (bind _returnvalue_4 (Rendering|Material|CreateDynamicMaterialInstance "/Game/Assets/Materials/M_BaseColor.M_BaseColor" "None" "None" :!class /Script/Engine.KismetMaterialLibrary))
      (Rendering|Material|SetVectorParameterValue _returnvalue_4 "Color" (.colordark _returnvalue) :!class /Script/Engine.MaterialInstanceDynamic)
      (Rendering|Material|SetMaterial (Variables|Character|GetMesh) 3 _returnvalue_4))))

(event EventTick
  (params (DeltaSeconds :type Float%20%28single-precision%29)))

(fn ConstructionScript)