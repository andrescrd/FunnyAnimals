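; Lobby game mode that manages joining and leaving players, shared map settings, kicking and launching the match.
; On login the server records the controller, reads server info from GI_GameInfoInstance, sets up PC_Lobby and replaces any existing pawn with a BP_Bird at a random PlayerStart.
; EveryoneUpdate pushes player counts, info and available characters to all controllers.
; Launch uses server travel to the map selected by ID; SwapCharacter is an empty stub.
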(event Custom|SwapCharacter
  (params (PlayerController :type Player%20Controller%20Object%20Reference) (CharacterClass :type Character%20Class%20Reference) (ChangedStatus :type Boolean)))

(event Custom|EveryoneUpdate
  (bind _allplayercontroller (Variables|ServerSetting|GetAllPlayerController))
  ;[1 1 1] update connected player information
  (bind _output_get (Variables|ServerSetting|SetCurrentPlayers (Utilities|Array|Length (Variables|ServerSetting|GetAllPlayerController))))
  (if (> _output_get 0)
    (Utilities|Array|Clear (Variables|ServerSetting|GetConnectedPlayers))
    (for _array_element _allplayercontroller
      (bind _aspc_lobby (Utilities|Casting|CastToPC_Lobby _array_element))
      (Utilities|Array|Add (Variables|ServerSetting|GetConnectedPlayers) (Variables|/Game/Blueprints/Lobby/PC_Lobby.PC_Lobby_C|GetPlayerInfo _aspc_lobby))
      (Default|UpdateNumberOfPlayers _aspc_lobby (Variables|ServerSetting|GetCurrentPlayers) (Variables|ServerSetting|GetMaxPlayers)))
    (for _array_element_2 _allplayercontroller
      (bind _aspc_lobby_2 (Utilities|Casting|CastToPC_Lobby _array_element_2))
      (Default|AddPlayerInfo _aspc_lobby_2 (Variables|ServerSetting|GetConnectedPlayers))
      (Default|UpdateAvailableCharacter _aspc_lobby_2 (Variables|Default|GetAvailableCharacter)))
    (Variables|ServerSetting|SetCanStart? true)))

(event Custom|LaunghGame
  (bind _returnvalue (Game|GetPlayerController 0))
  ;[1 1 1] Launch the game
  (switch int (Variables|ServerSetting|GetGM_MapID)
    (:Default
      (Development|ExecuteConsoleCommand "servertravel Map1" _returnvalue :!label _label))
    (:0
      (goto _label))
    (:1
      (Development|ExecuteConsoleCommand "servertravel  Map2" _returnvalue))))

(event Custom|RespawnPlayer
  (params (PlayerController :type Player%20Controller%20Object%20Reference))
  (bind _returnvalue (Pawn|GetControlledPawn PlayerController))
  (bind _playerspawn (Variables|ServerSetting|GetPlayerSpawn))
  ;[1 1 1] Spawn the player character
  (Utilities|IsValid _returnvalue
    (:Is%20Valid
      (Actor|DestroyActor _returnvalue)
      (bind _returnvalue_2 (Game|SpawnActorfromClass "/Game/Blueprints/Character/BP_Bird.BP_Bird_C" (Transformation|GetActorTransform (Utilities|Array|Get(acopy) _playerspawn (Math|Random|RandomIntegerinRange 0 (- (Utilities|Array|Length _playerspawn) 1)))) "Undefined" 0 0))
      (Pawn|Possess PlayerController _returnvalue_2)
      (CallFunction|EveryoneUpdate))))

(event Custom|ServerUpdateSetting
  (params (MapImage :type Texture%202D%20Object%20Reference) (MapName :type Text) (MapTime :type Text) (MapID :type Integer))
  ;[1 1 1] update changes made by the server
  (Variables|ServerSetting|SetGM_MapImage MapImage)
  (Variables|ServerSetting|SetGM_MapName MapName)
  (Variables|ServerSetting|SetGM_MapTime MapTime)
  (Variables|ServerSetting|SetGM_MapID MapID)
  (for _array_element (Variables|ServerSetting|GetAllPlayerController)
    (bind _aspc_lobby (Utilities|Casting|CastToPC_Lobby _array_element))
    (Default|UpdateLobbySetting _aspc_lobby (Variables|ServerSetting|GetGM_MapImage) (Variables|ServerSetting|GetGM_MapName) (Variables|ServerSetting|GetGM_MapTime))))

(event Custom|AddToKickList
  ;[1 1 1] Refresh the kicked list if it is open
  (bind _aspc_lobby (Utilities|Casting|CastToPC_Lobby (Game|GetPlayerController 0)))
  (Utilities|IsValid (Variables|/Game/Blueprints/Lobby/PC_Lobby.PC_Lobby_C|GetLobbyMenuWB _aspc_lobby)
    (:Is%20Valid
      (if (Widget|IsVisible (Variables|/Game/UI/Lobby/WB_LobbyMenu.WB_LobbyMenu_C|GetGameSetting (Variables|/Game/Blueprints/Lobby/PC_Lobby.PC_Lobby_C|GetLobbyMenuWB _aspc_lobby)))
        (Default|FillPlayersWindow (Variables|/Game/UI/Lobby/WB_LobbyMenu.WB_LobbyMenu_C|GetGameSetting (Variables|/Game/Blueprints/Lobby/PC_Lobby.PC_Lobby_C|GetLobbyMenuWB _aspc_lobby)))))))

(event Custom|YouHaveBeenKicked
  (params (PlayerID :type Integer))
  ;[1 1 1] Kick the selected player
  (bind _aspc_lobby (Utilities|Casting|CastToPC_Lobby (Utilities|Array|Get(acopy) (Variables|ServerSetting|GetAllPlayerController) PlayerID)))
  (Default|Kicked _aspc_lobby))

(event EventPostLogin
  (params (NewPlayer :type Player%20Controller%20Object%20Reference))
  ;[1 1 1] Initial setup event post login
  (Networking|SwitchHasAuthority
    (:Authority
      (Utilities|Array|Add (Variables|ServerSetting|GetAllPlayerController) NewPlayer)
      (bind _outactors (Actor|GetAllActorsOfClass "/Script/Engine.PlayerStart"))
      (Variables|ServerSetting|SetPlayerSpawn _outactors)
      (bind _asgi_game_info_instance (Utilities|Casting|CastToGI_GameInfoInstance (Game|GetGameInstance)))
      (Variables|ServerSetting|SetServerName (Variables|/Game/Blueprints/AllLevels/GI_GameInfoInstance.GI_GameInfoInstance_C|GetServerName _asgi_game_info_instance))
      (Variables|ServerSetting|SetMaxPlayers (Variables|/Game/Blueprints/AllLevels/GI_GameInfoInstance.GI_GameInfoInstance_C|GetMaxPlayers _asgi_game_info_instance))
      (bind _aspc_lobby (Utilities|Casting|CastToPC_Lobby NewPlayer))
      (Default|InitialSetup _aspc_lobby)
      (Default|SetupLobbyMenu _aspc_lobby (Variables|ServerSetting|GetServerName))
      (Default|UpdateLobbySetting _aspc_lobby (Variables|ServerSetting|GetGM_MapImage) (Variables|ServerSetting|GetGM_MapName) (Variables|ServerSetting|GetGM_MapTime))
      (Default|UpdateNumberOfPlayers _aspc_lobby (Variables|ServerSetting|GetCurrentPlayers) (Variables|ServerSetting|GetMaxPlayers))
      (CallFunction|RespawnPlayer NewPlayer))))

(event EventOnLogout
  (params (ExitingController :type Controller%20Object%20Reference))
  ;[1 1 1] Logout player and update all
  (bind (_array_element _array_index) (Utilities|Array|ForEachLoopwithBreak (Variables|ServerSetting|GetAllPlayerController) :!label _label)
    (:LoopBody
      (if (== _array_element ExitingController)
        (goto _label Break)))
    (:Completed
      (Utilities|Array|RemoveIndex (Variables|ServerSetting|GetAllPlayerController) _array_index)
      (Utilities|Array|RemoveIndex (Variables|ServerSetting|GetConnectedPlayers) _array_index)
      (CallFunction|EveryoneUpdate))))

(fn ConstructionScript)